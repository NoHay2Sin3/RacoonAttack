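; BP_Racoon_Placeholder is a placeholder raccoon character with camera-relative movement, look and jump input.
; When CanInteractBoc is true, Empujar toggles box pushing, switching walk speed and physics simulation on the Cubo_Empujable found at BeginPlay.
; The push box overlap only prints and sets a flag, as its impulse code is disconnected.
; Author notes mark both push attempts as discarded or failed.
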(event OnComponentBeginOverlap(BoxCollision_Empujar)
  (params (OverlappedComponent :type Primitive%20Component%20Object%20Reference) (OtherActor :type Actor%20Object%20Reference) (OtherComp :type Primitive%20Component%20Object%20Reference) (OtherBodyIndex :type Integer) (bFromSweep :type Boolean) (SweepResult :type Hit%20Result%20Structure%20%28by%20ref%29))
  ;[1 1 1] Add impulse y add force fallido, no entiendo como funcionan bien las fisicas para que acabe funcionando
  (Development|PrintString (Utilities|GetDisplayName OverlappedComponent))
  (bind _output_get (Variables|Default|SetOverlap true)))

(event EventBeginPlay
  ;[1 1 1] Emujar descartado por el mismo problema que en el cubo, no reconoce la variable axis value
  (bind _returnvalue (Actor|GetActorOfClass "/Game/Personaje_Y_Movimiento/Cubo_Empujable.Cubo_Empujable_C"))
  (Variables|Default|Setcubo_empujable _returnvalue))

(event Input|ActionEvents|InputActionSaltar
  (params (Key :type Key%20Structure :default "None"))
  ;[0 0 0] Saltar
  (:Pressed
    (Character|Jump)))

(event Input|ActionEvents|InputActionEmpujar
  (params (Key :type Key%20Structure :default "None"))
  (bind _cubo_empujable (Variables|Default|Getcubo_empujable))
  (bind _sm_cubo_empujable (Variables|/Game/Personaje_Y_Movimiento/Cubo_Empujable.Cubo_Empujable_C|Getsm_cubo_empujable _cubo_empujable))
  ;[1 1 1] Emujar descartado por el mismo problema que en el cubo, no reconoce la variable axis value
  (:Pressed
    (if (Variables|Default|Getcan_interact_Boc)
      (if (Variables|Default|Getbox_interac)
        (Variables|Default|Setbox_interac false)
        (Variables|/Script/Engine.CharacterMovementComponent|SetMaxWalkSpeed (Variables|Character|GetCharacterMovement) 2.3e+02)
        (Physics|SetSimulatePhysics _sm_cubo_empujable false)
        (else
          (Variables|Default|Setbox_interac true)
          (Variables|/Script/Engine.CharacterMovementComponent|SetMaxWalkSpeed (Variables|Character|GetCharacterMovement) 6e+01)
          (Physics|SetSimulatePhysics _sm_cubo_empujable true))))))

(event Input|AxisEvents|InputAxisAdelante_Atras
  (params (AxisValue :type Float%20%28single-precision%29))
  ;[0 0 0] Movimiento - Adelante y Atras
  (bind _output_get (Variables|Default|SetAxis_Value_AdelanteAtras AxisValue))
  (Pawn|Input|AddMovementInput (Math|Vector|GetForwardVector (Pawn|GetControlRotation :!class /Script/Engine.Pawn)) _output_get false))

(event Input|AxisEvents|InputAxisDerecha_Izquierda
  (params (AxisValue :type Float%20%28single-precision%29))
  ;[0 0 0] Movimiento - Izquierda y Derecha
  (bind _output_get (Variables|Default|SetAxis_Value_IzquierdaDerecha AxisValue))
  (Pawn|Input|AddMovementInput (Math|Vector|GetRightVector (Pawn|GetControlRotation :!class /Script/Engine.Pawn)) _output_get false))

(event Input|AxisEvents|InputAxisMirar_Arriba_Abajo
  (params (AxisValue :type Float%20%28single-precision%29))
  ;[0 0 0] Camara - Arriba y Abajo
  (Pawn|Input|AddControllerPitchInput AxisValue))

(event Input|AxisEvents|InputAxisMirar_Izquierda_Derecha
  (params (AxisValue :type Float%20%28single-precision%29))
  ;[0 0 0] Camara - Izquierda y Derecha
  (Pawn|Input|AddControllerYawInput AxisValue))

(fn ConstructionScript)